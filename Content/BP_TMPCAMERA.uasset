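; Temporary camera actor, judging by its name, that pans slightly to follow the player's sideways position.
; Each Tick calls RotateCamera, which sets the Camera component's world rotation with a fixed downward pitch and zero roll.
; Yaw is an unclamped Lerp over a narrow angle range, driven by player pawn 0's world Y, scaled and offset.
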(event EventBeginPlay)

(event Collision|EventActorBeginOverlap
  (params (OtherActor :type Actor%20Object%20Reference)))

(event EventTick
  (params (DeltaSeconds :type Float%20%28single-precision%29))
  (CallFunction|RotateCamera))

(fn ConstructionScript)

(fn RotateCamera
  (Transformation|SetWorldRotation (Variables|Default|GetCamera) (Math|Rotator|MakeRotator 0.0 -3e+01 (Math|Float|Lerp -3.0 3.0 (+ (/ (.Y (Math|Vector|BreakVector (Transformation|GetActorLocation (Game|Player|GetPlayerPawn 0)))) 9e+02) 1.0))) false false))